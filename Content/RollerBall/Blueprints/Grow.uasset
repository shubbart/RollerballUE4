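; Grow pickup for the RollerBall game that makes the player's ball larger and heavier.
; On overlap with a RollerballPawn, it sets the sphere's scale and mass scale to fixed higher values, cuts the pawn's Vel to a small fraction, then destroys itself.
; Its Cube rotates by a fixed step every tick, independent of delta time.
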(event EventBeginPlay)

(event Collision|EventActorBeginOverlap
  (params (OtherActor :type Actor%20Object%20Reference))
  (bind _asrollerball_pawn (Utilities|Casting|CastToRollerballPawn OtherActor))
  (Transformation|SetRelativeScale3D (Variables|/Game/RollerBall/Blueprints/RollerballPawn.RollerballPawn_C|GetSphere _asrollerball_pawn) "1.500000,1.500000,1.500000")
  (Class|PrimitiveComponent|SetMassScale (Variables|/Game/RollerBall/Blueprints/RollerballPawn.RollerballPawn_C|GetSphere _asrollerball_pawn) "None" 1.25)
  (Variables|/Game/RollerBall/Blueprints/RollerballPawn.RollerballPawn_C|SetVel _asrollerball_pawn (* (Variables|/Game/RollerBall/Blueprints/RollerballPawn.RollerballPawn_C|GetVel _asrollerball_pawn) 0.05))
  (Actor|DestroyActor))

(event EventTick
  (params (DeltaSeconds :type Float%20%28single-precision%29))
  (Transformation|AddLocalRotation (Variables|Default|GetCube) "0.500000,0.500000,0.500000" false false))

(fn ConstructionScript)