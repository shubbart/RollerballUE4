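; Rollerball player pawn that the player steers by pushing a physics sphere around.
; Horizontal and Vertical axis inputs apply world-space forces along X and Y to the Sphere component, scaled by the Vel variable.
; BeginPlay sets Vel and stores a copy in VelReset, which this Blueprint never reads back.
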(event EventBeginPlay
  (bind _output_get (Variables|Default|SetVel 1.5e+04))
  (Variables|Default|SetVelReset _output_get))

(event EventTick
  (params (DeltaSeconds :type Float%20%28single-precision%29)))

(event Input|AxisEvents|InputAxisHorizontal
  (params (AxisValue :type Float%20%28single-precision%29))
  (Physics|AddForce (Variables|Default|GetSphere) (Math|Vector|MakeVector (* AxisValue (Variables|Default|GetVel)) 0.0 0.0) "None" false))

(event Input|AxisEvents|InputAxisVertical
  (params (AxisValue :type Float%20%28single-precision%29))
  (Physics|AddForce (Variables|Default|GetSphere) (Math|Vector|MakeVector 0.0 (* AxisValue (Variables|Default|GetVel)) 0.0) "None" false))

(fn ConstructionScript)