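; Teleporter actor for RollerBall that moves the player's rollerball to a linked Destination.
; On overlap while IsActive, it casts the other actor to RollerballPawn and sets its Sphere component to the Destination root's world location, without sweep or the teleport physics flag.
; Tick spins the Cube by a fixed step each frame, so its speed depends on frame rate.
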(event EventBeginPlay)

(event Collision|EventActorBeginOverlap
  (params (OtherActor :type Actor%20Object%20Reference))
  (if (Variables|Default|GetisActive)
    (bind _asrollerball_pawn (Utilities|Casting|CastToRollerballPawn OtherActor))
    (Transformation|SetWorldLocation (Variables|/Game/RollerBall/Blueprints/RollerballPawn.RollerballPawn_C|GetSphere _asrollerball_pawn) (Transformation|GetWorldLocation (Variables|/Script/Engine.Actor|GetRootComponent (Variables|Default|GetDestination))) false false)))

(event EventTick
  (params (DeltaSeconds :type Float%20%28single-precision%29))
  (Transformation|AddLocalRotation (Variables|Default|GetCube) "0.000000,1.000000,0.000000" false false))

(fn ConstructionScript)